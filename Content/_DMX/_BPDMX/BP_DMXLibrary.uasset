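; BP_DMXLibrary is a utility Blueprint that bulk-creates and removes RGB fixture patches in a DMX library.
; When CreateFixture is set, BeginPlay loops over universes and LEDs, adding patches at three-channel address intervals.
; It stores the patch references in a BP_SaveFixtureArray save slot.
; When RemoveFixture is set, EndPlay reloads that slot, removes the saved patches from the library and deletes the save.
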(event EventBeginPlay
  (if (Variables|Default|GetCreateFixture)
    (for _index (range 0 (- (Variables|Default|GetUniverse) 1))
      (for _index_2 (range 0 (- (Variables|Default|GetNumberofLED) 1))
        (bind _returnvalue (Class|DMXEntityFixturePatch|CreateFixturePatchinLibrary (Utilities|Struct|MakeDMXEntityFixturePatchConstructionParams "(DMXLibrary=\"/Script/DMXRuntime.DMXLibrary'/Game/_DMX/DMX_Tutorial.DMX_Tutorial'\",bDisplayLibraryPicker=True,EntityType=\"/Script/CoreUObject.Class'/Script/DMXRuntime.DMXEntityFixtureType'\",EntityId=3DBE320C48337C86F188039D390E9EBA)" (+ _index 1) (+ (* _index_2 3) 1)) "RGB" false))
        (Utilities|Array|Add (Variables|Default|GetFixtureArray) _returnvalue)))
    (bind _returnvalue_2 (SaveGame|CreateSaveGameObject "/Game/_DMX/_BPDMX/BP_SaveFixtureArray.BP_SaveFixtureArray_C"))
    (bind _output_get (Variables|Default|SetSave%20REF _returnvalue_2))
    (Variables|/Game/_DMX/_BPDMX/BP_SaveFixtureArray.BP_SaveFixtureArray_C|SetSavedFixtureArray _output_get (Variables|Default|GetFixtureArray))
    (SaveGame|SaveGametoSlot (Variables|Default|GetSave%20REF) "FixtureArray")))

(event EventEndPlay
  (params (EndPlayReason :type EEndPlayReason%20Enum :default "Destroyed"))
  (if (Variables|Default|GetRemoveFixture)
    (bind _returnvalue (SaveGame|LoadGamefromSlot "FixtureArray"))
    (bind _asbp_save_fixture_array (Utilities|Casting|CastToBP_SaveFixtureArray _returnvalue))
    (for _array_element (Variables|/Game/_DMX/_BPDMX/BP_SaveFixtureArray.BP_SaveFixtureArray_C|GetSavedFixtureArray _asbp_save_fixture_array)
      (Class|DMXEntityFixturePatch|RemoveFixturePatchfromLibrary (Class|DMXEntityReferenceConversions|ToRef(FixturePatchObj) _array_element)))
    (Utilities|Array|RemoveItem (Variables|/Game/_DMX/_BPDMX/BP_SaveFixtureArray.BP_SaveFixtureArray_C|GetSavedFixtureArray _asbp_save_fixture_array) 0)
    (SaveGame|DeleteGameinSlot "FixtureArray")))

(fn ConstructionScript)
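; BP_LEDTest_144s_1m is a DMX-driven LED test fixture actor that sets the color of an LED component from incoming DMX data.
; On BeginPlay it assigns its fixture patch to the DMX component and creates a dynamic instance of M_LED on the LED.
; Each received patch update reads normalized attribute values and writes three of them as RGB into the material's DMXColor vector parameter.
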(event OnFixturePatchReceived(DMX)
  (params (FixturePatch :type DMX%20Entity%20Fixture%20Patch%20Object%20Reference) (ValuePerAttribute :type DMX%20Normalized%20Attribute%20Value%20Map%20Structure%20%28by%20ref%29))
  (bind _normalizedattributesvalues (Class|DMXEntityFixturePatch|GetNormalizedAttributesValues FixturePatch))
  (Rendering|Material|SetVectorParameterValue (Variables|Default|GetLEDColor) "DMXColor" (Utilities|Struct|MakeLinearColor (.Value (Utilities|Map|Find (.map _normalizedattributesvalues) "(Name=\"Red\")")) (.Value (Utilities|Map|Find (.map _normalizedattributesvalues) "(Name=\"Green\")")) (.Value (Utilities|Map|Find (.map _normalizedattributesvalues) "(Name=\"Blue\")")) 0.0) :!class /Script/Engine.MaterialInstanceDynamic))

(event EventBeginPlay
  (Class|DMXComponent|SetFixturePatch (Variables|Default|GetDMX) (Variables|Default|GetSetFixture))
  (bind _returnvalue (Rendering|Material|CreateDynamicMaterialInstance (Variables|Default|GetLED) 0 "/Game/_DMX/_MAT/M_LED.M_LED" "None" :!class /Script/Engine.PrimitiveComponent))
  (Variables|Default|SetLEDColor _returnvalue))

(fn ConstructionScript)
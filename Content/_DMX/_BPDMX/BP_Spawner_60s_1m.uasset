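; Spawner Blueprint that builds a run of BP_LEDTest_60s_1m LED actors for one DMX universe at play start.
; BeginPlay removes the tape and LED viewport components, then waits in proportion to Universe, staggering spawners by universe.
; It then spawns NumberofLED actors at SpawnLocation offsets from the root, copying its rotation and scale.
; Each actor receives the Universe and a starting address three channels after the previous one.
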(event EventBeginPlay
  (bind _defaultsceneroot (Variables|Default|GetDefaultSceneRoot))
  (bind _returnvalue (Transformation|GetWorldTransform _defaultsceneroot))
  (Components|DestroyComponent (Variables|Default|GetTapeViewPort))
  (Components|DestroyComponent (Variables|Default|GetLEDViewPort))
  (Utilities|FlowControl|Delay (* (Variables|Default|GetUniverse) 0.1))
  (for _index (range 0 (- (Variables|Default|GetNumberofLED) 1))
    (Game|SpawnActorfromClass "/Game/_DMX/_BPDMX/BP_LEDTest_60s_1m.BP_LEDTest_60s_1m_C" (Math|Transform|MakeTransform (+ (|SpawnLocation _index) (.location _returnvalue)) (.rotation _returnvalue) (.scale _returnvalue)) "Undefined" "MultiplyWithRoot" 0 (Variables|Default|GetUniverse) (+ (* _index 3) 1) 0)))

(fn ConstructionScript)
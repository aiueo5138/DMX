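; DMX-driven LED test Blueprint that shows color received from a DMX fixture patch on its LED component.
; On BeginPlay it creates an RGB fixture patch at its Universe and StartingAddress, assigns it to the DMX component, and makes a dynamic M_LED material.
; Each received patch update writes normalized attribute values into the material's DMXColor parameter.
; EndPlay removes the runtime-created patch from the library.
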(event OnFixturePatchReceived(DMX)
  (params (FixturePatch :type DMX%20Entity%20Fixture%20Patch%20Object%20Reference) (ValuePerAttribute :type DMX%20Normalized%20Attribute%20Value%20Map%20Structure%20%28by%20ref%29))
  (bind _normalizedattributesvalues (Class|DMXEntityFixturePatch|GetNormalizedAttributesValues FixturePatch))
  (Rendering|Material|SetVectorParameterValue (Variables|Default|GetLEDColor) "DMXColor" (Utilities|Struct|MakeLinearColor (.Value (Utilities|Map|Find (.map _normalizedattributesvalues) "(Name=\"Red\")")) (.Value (Utilities|Map|Find (.map _normalizedattributesvalues) "(Name=\"Green\")")) (.Value (Utilities|Map|Find (.map _normalizedattributesvalues) "(Name=\"Blue\")")) 0.0) :!class /Script/Engine.MaterialInstanceDynamic))

(event EventBeginPlay
  (bind _returnvalue (Class|DMXEntityFixturePatch|CreateFixturePatchinLibrary (Utilities|Struct|MakeDMXEntityFixturePatchConstructionParams "(DMXLibrary=\"/Script/DMXRuntime.DMXLibrary'/Game/_DMX/DMX_Tutorial.DMX_Tutorial'\",bDisplayLibraryPicker=True,EntityType=\"/Script/CoreUObject.Class'/Script/DMXRuntime.DMXEntityFixtureType'\",EntityId=3DBE320C48337C86F188039D390E9EBA)" (Variables|Default|GetUniverse) (Variables|Default|GetStarting%20Address)) "RGB" false))
  (Class|DMXComponent|SetFixturePatch (Variables|Default|GetDMX) _returnvalue)
  (bind _returnvalue_2 (Rendering|Material|CreateDynamicMaterialInstance (Variables|Default|GetLED) 0 "/Game/_DMX/_MAT/M_LED.M_LED" "None" :!class /Script/Engine.PrimitiveComponent))
  (Variables|Default|SetLEDColor _returnvalue_2))

(event EventEndPlay
  (params (EndPlayReason :type EEndPlayReason%20Enum :default "Destroyed"))
  (Class|DMXEntityFixturePatch|RemoveFixturePatchfromLibrary (Class|DMXEntityReferenceConversions|ToRef(FixturePatchObj) (Class|DMXComponent|GetFixturePatch (Variables|Default|GetDMX)))))

(fn ConstructionScript)
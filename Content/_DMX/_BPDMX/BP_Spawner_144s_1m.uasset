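; Spawner for one DMX universe of 144s_1m LED test actors, each bound to a saved fixture.
; On BeginPlay it removes its viewport preview components, then waits in proportion to its Universe number, staggering spawners.
; It loads the FixtureArray save game and spawns NumberofLED actors at SpawnLocation offsets from its root transform, passing each the fixture from that universe's slice of the saved array.
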(event EventBeginPlay
  (bind _defaultsceneroot (Variables|Default|GetDefaultSceneRoot))
  (bind _returnvalue (Transformation|GetWorldTransform _defaultsceneroot))
  (Components|DestroyComponent (Variables|Default|GetTapeViewPort))
  (Components|DestroyComponent (Variables|Default|GetLEDViewPort))
  (Utilities|FlowControl|Delay (* (Variables|Default|GetUniverse) 0.1))
  (bind _returnvalue_2 (SaveGame|DoesSaveGameExist "FixtureArray"))
  (if _returnvalue_2
    (bind _returnvalue_3 (SaveGame|LoadGamefromSlot "FixtureArray"))
    (bind _asbp_save_fixture_array (Utilities|Casting|CastToBP_SaveFixtureArray _returnvalue_3))
    (for _index (range 0 (- (Variables|Default|GetNumberofLED) 1))
      (Game|SpawnActorfromClass "/Game/_DMX/_BPDMX/BP_LEDTest_144s_1m.BP_LEDTest_144s_1m_C" (Math|Transform|MakeTransform (+ (|SpawnLocation _index) (.location _returnvalue)) (.rotation _returnvalue) (.scale _returnvalue)) "Undefined" "MultiplyWithRoot" 0 (Utilities|Array|Get(acopy) (Variables|/Game/_DMX/_BPDMX/BP_SaveFixtureArray.BP_SaveFixtureArray_C|GetSavedFixtureArray _asbp_save_fixture_array) (+ _index (* (Variables|Default|GetNumberofLED) (- (Variables|Default|GetUniverse) 1)))) 0))))

(fn ConstructionScript)